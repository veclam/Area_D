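; Door Blueprint that opens or closes on interaction only when it is unlocked and the passed object types contain its needed item.
; A timeline lerps the Cube between its starting and desired rotations, playing or reversing by IsOpen, which flips when it finishes.
; A locked or missing-item attempt plays a slight yaw animation instead.
; Overlapping either box reverses the door timeline while IsOpen is false.
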(event `self.ReceiveBeginPlay`
  (`parent.ReceiveBeginPlay`)
  (set `self.origineRotation` (`SceneComponent.K2_GetComponentRotation` (`self.Cube`))))

(event `/Game/developement/BP/parentObject/MasterObject/BP_parentObject.interactWithObject`
  (params (objectType :type "Array of /Game/developement/data/E_ObjectType Enum (by ref)" :default _))
  (bind (_originerotation_roll _originerotation_pitch _originerotation_yaw) (`KismetMathLibrary.BreakRotator` (`self.origineRotation`)))
  (if (or (`self.isLocked`) (not (`KismetArrayLibrary.Array_Contains` objectType (`self.neededItem`))))
    (bind (_direction _newtrack_0) (`Timeline|lockedDoorAnim` :!via `PlayFromStart`)
      (:`Update`
        (`SceneComponent.K2_SetWorldRotation` (`self.Cube`) (`KismetMathLibrary.RLerp` (`self.origineRotation`) (`KismetMathLibrary.MakeRotator` _originerotation_roll _originerotation_pitch (+ _originerotation_yaw 1.0)) _newtrack_0) false false)))
    (elif (`self.isOpen`)
      (bind (_direction_2 _newtrack_0_2) (`Timeline|open/closeDoor` :!label _label)
        (:`Update`
          (`SceneComponent.K2_SetWorldRotation` (`self.Cube`) (`KismetMathLibrary.RLerp` (`self.origineRotation`) (`self.desiredRotation`) _newtrack_0_2) false false))
        (:`Finished`
          (set `self.isOpen` (not (`self.isOpen`)))))
      (else
        (goto _label :!via `Reverse`)))))

(event `self.Box.OnComponentBeginOverlap`
  (params (OverlappedComponent :type "PrimitiveComponent Object Reference") (OtherActor :type "Actor Object Reference") (OtherComp :type "PrimitiveComponent Object Reference") (OtherBodyIndex :type Integer) (bFromSweep :type Boolean) (SweepResult :type "HitResult Structure (by ref)"))
  (if (not (`self.isOpen`)) :!label _label_2
    (goto _label :!via `Reverse`)))

(event `self.Box1.OnComponentBeginOverlap`
  (params (OverlappedComponent :type "PrimitiveComponent Object Reference") (OtherActor :type "Actor Object Reference") (OtherComp :type "PrimitiveComponent Object Reference") (OtherBodyIndex :type Integer) (bFromSweep :type Boolean) (SweepResult :type "HitResult Structure (by ref)"))
  (goto _label_2))

(fn `UserConstructionScript`
  (`parent.UserConstructionScript`))