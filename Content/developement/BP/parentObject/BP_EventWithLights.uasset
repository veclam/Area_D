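; BP_EventWithLights is a parent trigger object that fades a set of referenced lights to a target intensity when something overlaps its box.
; The first overlap runs once, caching each light's current intensity in BaseIntensity.
; The AnimLights timeline then lerps every light in RefLights from its cached value to WantedLightsIntensity on each update.
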(event `self.Box.OnComponentBeginOverlap`
  (params (OverlappedComponent :type "PrimitiveComponent Object Reference") (OtherActor :type "Actor Object Reference") (OtherComp :type "PrimitiveComponent Object Reference") (OtherBodyIndex :type Integer) (bFromSweep :type Boolean) (SweepResult :type "HitResult Structure (by ref)"))
  (`/Engine/EditorBlueprintResources/StandardMacros.DoOnce` false
    (:`Completed`
      (for _array_element (`self.refLights`)
        (`KismetArrayLibrary.Array_Add` (`self.baseIntensity`) (`LightComponentBase.Intensity` (`Light.LightComponent` _array_element))))
      (bind (_direction _newtrack_0) (`Timeline|animLights`)
        (:`Update`
          (for (_array_element_2 _array_index) (`self.refLights`)
            (`LightComponent.SetIntensity` (`Light.LightComponent` _array_element_2) (`KismetMathLibrary.Lerp` (`|GetArrayItem` (`self.baseIntensity`) _array_index) (`self.wantedLightsIntensity`) _newtrack_0))))))))

(fn `UserConstructionScript`
  (`parent.UserConstructionScript`))