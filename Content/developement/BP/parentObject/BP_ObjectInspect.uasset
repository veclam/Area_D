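; BP_ObjectInspect is an inspectable object, apparently a parent class, that moves up in front of the player and back.
; It caches its transform on BeginPlay; Inspect stores the target location, fires inspectObj and returns itself.
; A FlipFlop alternates two timelines that lerp the transform to that location, keeping rotation and scale, or back to the origin.
; An author note flags the FlipFlop as fragile, preferring a bool.
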(event `self.ReceiveBeginPlay`
  (`parent.ReceiveBeginPlay`)
  (set `self.OrigineTransform` (`self.GetTransform`)))

(event `inspectObj`
  (bind (_originetransform_location _originetransform_rotation _originetransform_scale) (`KismetMathLibrary.BreakTransform` (`self.OrigineTransform`)))
  ; faire attantion au flip flop mettre plutot un bool
  (`/Engine/EditorBlueprintResources/StandardMacros.FlipFlop`
    (:`A`
      ; select pour la translation permet de supr une timeline
      (bind (_direction _take) (`Timeline|Timeline_Take` :!via `PlayFromStart`)
        (:`Update`
          (`self.K2_SetActorTransform` (`KismetMathLibrary.TLerp` (`self.OrigineTransform`) (`KismetMathLibrary.MakeTransform` (`self.frontPlayer`) _originetransform_rotation _originetransform_scale) _take)))))
    (:`B`
      (bind (_direction_2 _dropobject) (`Timeline|Timeline_0` :!via `PlayFromStart`)
        (:`Update`
          (`self.K2_SetActorTransform` (`KismetMathLibrary.TLerp` (`self.GetTransform`) (`self.OrigineTransform`) _dropobject)))))))

(fn `inspect`
  (params (frontPlayer :type "Vector Structure"))
  (returns (succes :type Boolean) (objectToInspect :type "Actor Object Reference"))
  (set `self.frontPlayer` frontPlayer)
  (`self.inspectObj`)
  (return true self))

(fn `UserConstructionScript`
  (`parent.UserConstructionScript`))