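; Parent Blueprint, by name and folder, for objects whose interaction depends on a required object.
; Its InteractwithObject event scans the supplied ObjectType array for NeededObject and sets the DoSMTH flag on a match.
; The branch on that flag is empty, so a match triggers no action here, and the flag is never reset.
; BeginPlay, overlap and Tick are disabled stubs.
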(event `self.interactWithObject`
  (params (objectType :type "Array of /Game/developement/data/E_ObjectType Enum (by ref)" :default _))
  (if (> (`KismetArrayLibrary.Array_Length` objectType) 0)
    (for _array_element objectType
      (if (`|EnumEquality` _array_element (`self.neededObject`))
        (set `self.DoSMTH` true)))
    (if (`self.DoSMTH`)
      _)))

(fn `UserConstructionScript`
  (`parent.UserConstructionScript`))