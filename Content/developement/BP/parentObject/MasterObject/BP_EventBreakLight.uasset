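; Trigger actor that, judging by its name, stages a breaking-light event when its Box is first overlapped.
; A DoOnce limits the response to a single firing, with no check on which actor overlaps.
; It sets each light in the Light array to a new intensity, then swaps material slot 1 on each actor in the Mesh array to the Materials material.
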(event `self.Box.OnComponentBeginOverlap`
  (params (OverlappedComponent :type "PrimitiveComponent Object Reference") (OtherActor :type "Actor Object Reference") (OtherComp :type "PrimitiveComponent Object Reference") (OtherBodyIndex :type Integer) (bFromSweep :type Boolean) (SweepResult :type "HitResult Structure (by ref)"))
  (`/Engine/EditorBlueprintResources/StandardMacros.DoOnce` false
    (:`Completed`
      (for _array_element (`self.light`)
        (`LightComponent.SetIntensity` (`Light.LightComponent` _array_element) (`self.New Intensity`)))
      (for _array_element_2 (`self.mesh`)
        (`PrimitiveComponent.SetMaterial` (`StaticMeshActor.StaticMeshComponent` _array_element_2) 1 (`self.materials`))))))

(fn `UserConstructionScript`
  (`parent.UserConstructionScript`))