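; BP_FuseBox is an interactable fuse box that changes the intensity of a set of referenced lights, once.
; On its first InteractwithObject event, it records each light's current intensity in an array.
; A Timeline then lerps every light from its recorded value to a shared target intensity, using the array index to match each light to its starting value.
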(event `/Game/FirstPerson/Blueprints/BPI_interact.interactWithObject`
  (params (objectType :type "Array of /Game/developement/data/E_ObjectType Enum (by ref)" :default _))
  (`/Engine/EditorBlueprintResources/StandardMacros.DoOnce` false
    (:`Completed`
      (for _array_element (`self.lightsRef`)
        (`KismetArrayLibrary.Array_Add` (`self.baseIntensity`) (`LightComponentBase.Intensity` (`Light.LightComponent` _array_element))))
      (bind (_direction _newtrack_0) (`Timeline|Timeline`)
        (:`Update`
          (for (_array_element_2 _array_index) (`self.lightsRef`)
            (`LightComponent.SetIntensity` (`Light.LightComponent` _array_element_2) (`KismetMathLibrary.Lerp` (`|GetArrayItem` (`self.baseIntensity`) _array_index) (`self.wantedLightsIntensity`) _newtrack_0))))))))

(fn `UserConstructionScript`
  (`parent.UserConstructionScript`))