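; BP_TV is an interactable television actor that turns on its screens to show video materials.
; On InteractwithObject, it loops over six screen meshes, including EcranCasser (broken screen), unhides each one and sets its first material to the ListVideo entry at the same index.
; The event only switches screens on; BeginPlay, overlap and Tick are disabled stubs, and the construction script just calls its parent.
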(event `/Game/FirstPerson/Blueprints/BPI_interact.interactWithObject`
  (params (objectType :type "Array of /Game/developement/data/E_ObjectType Enum (by ref)" :default _))
  (for (_array_element _array_index) (`|MakeArray` (`self.Plane`) (`self.Plane1`) (`self.Plane2`) (`self.Plane3`) (`self.EcranCasser`) (`self.Plane5`))
    (`SceneComponent.SetHiddenInGame` _array_element false false)
    (`PrimitiveComponent.SetMaterial` _array_element 0 (`|GetArrayItem` (`self.listVideo`) _array_index))))

(fn `UserConstructionScript`
  (`parent.UserConstructionScript`))