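; Broken camera Blueprint that the player repairs by interacting with it using a specific object type.
; A looping timer set on BeginPlay periodically activates the Electricity spark effect while the camera is broken.
; The first matching interaction pauses that timer and plays a timeline that blends the actor's current transform toward RepairedTransform, then sets HisRepaired when finished.
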(event `self.ReceiveBeginPlay`
  (`parent.ReceiveBeginPlay`)
  (bind _returnvalue (`KismetSystemLibrary.K2_SetTimerDelegate` (delegate `etincelle`) 10.0 true))
  (set `self.timerNiagara` _returnvalue))

(event `etincelle`
  (`ActorComponent.Activate` (`self.electricity`) true))

(event `/Game/FirstPerson/Blueprints/BPI_interact.interactWithObject`
  (params (objectType :type "Array of /Game/developement/data/E_ObjectType Enum (by ref)" :default _))
  (if (`KismetArrayLibrary.Array_Contains` objectType "NewEnumerator2")
    (`/Engine/EditorBlueprintResources/StandardMacros.DoOnce` false
      (:`Completed`
        (`KismetSystemLibrary.K2_PauseTimerHandle` (`self.timerNiagara`))
        (bind (_direction _newtrack_0) (`Timeline|Timeline_0`)
          (:`Update`
            (`self.K2_SetActorTransform` (`KismetMathLibrary.TLerp` (`self.GetTransform`) (`self.RepairedTransform`) _newtrack_0)))
          (:`Finished`
            (set `self.HisRepaired` true)))))))

(fn `UserConstructionScript`
  (`parent.UserConstructionScript`))