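; BP_doorEnd is an interactable end door that finishes the game when the player uses it.
; Its InteractwithObject event creates the WG_end widget and adds it to the viewport.
; After a fixed delay it opens the main menu level; the default BeginPlay, overlap and Tick events are disabled.
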(event `/Game/FirstPerson/Blueprints/BPI_interact.interactWithObject`
  (params (objectType :type "Array of /Game/developement/data/E_ObjectType Enum (by ref)" :default _))
  (bind _returnvalue (`|CreateWidget` "/Game/developement/BP/widget/WG_end.WG_end_C"))
  (`UserWidget.AddToViewport` _returnvalue 0)
  (`KismetSystemLibrary.Delay` 10.0)
  (`GameplayStatics.OpenLevelBySoftObjectPtr` "/Game/FirstPerson/Lvl_mainMenu.Lvl_mainMenu"))

(fn `UserConstructionScript`
  (`parent.UserConstructionScript`))