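; BP_door is an interactable door actor that toggles between open and closed by rotating its Cube component.
; BeginPlay stores the cube's world rotation as the origin.
; Each InteractwithObject call alternates through a FlipFlop between playing and reversing the OpencloseDoor timeline.
; The timeline track drives a rotator lerp from that origin to DesiredRotation, applied as the cube's world rotation.
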(event `self.ReceiveBeginPlay`
  (`parent.ReceiveBeginPlay`)
  (set `self.origineRotation` (`SceneComponent.K2_GetComponentRotation` (`self.Cube`))))

(event `/Game/FirstPerson/Blueprints/BPI_interact.interactWithObject`
  (params (objectType :type "Array of /Game/developement/data/E_ObjectType Enum (by ref)" :default _))
  (`/Engine/EditorBlueprintResources/StandardMacros.FlipFlop`
    (:`A`
      (bind (_direction _newtrack_0) (`Timeline|open/closeDoor` :!label _label)
        (:`Update`
          (`SceneComponent.K2_SetWorldRotation` (`self.Cube`) (`KismetMathLibrary.RLerp` (`self.origineRotation`) (`self.desiredRotation`) _newtrack_0) false false))))
    (:`B`
      (goto _label :!via `Reverse`))))

(fn `UserConstructionScript`
  (`parent.UserConstructionScript`))